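; BP_Enemy is an AI enemy that relays Pawn Sensing sight and hearing events to the AIController_BP_Hunter blackboard.
; Heard noises set LastHeardLocation with a debug sphere, and a timer clears it after a few seconds.
; Seeing a player-controlled pawn sets EnemyActor and HasLOS.
; A vision-memory timer, restarted on each sighting, resets both keys when it expires.
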(event `self.PawnSensing.OnHearNoise`
  (params (Instigator :type "Pawn Object Reference") (Location :type "Vector Structure (by ref)") (Volume :type "Float (single-precision)"))
  (bind _asaicontroller_bp_hunter (cast `/Game/Blueprints/AI/AIController_BP_Hunter` (`self.GetController`)))
  (bind _output_get (set `self.HunterController` _asaicontroller_bp_hunter))
  (`BlackboardComponent.SetValueAsVector` (`AIBlueprintHelperLibrary.GetBlackboard` _output_get) (`self.LastHeardLocation`) Location)
  (`KismetSystemLibrary.DrawDebugSphere` Location 25.0 12 (struct :`R` 1.0 :`G` 0.031298 :`A` 1.0) 1.5)
  (`KismetSystemLibrary.K2_ClearAndInvalidateTimerHandle` (stale _returnvalue))
  (bind _returnvalue (`KismetSystemLibrary.K2_SetTimer` null "ClearHeard" 4.0)))

(event `self.PawnSensing.OnSeePawn`
  (params (Pawn :type "Pawn Object Reference"))
  (if (`self.IsPlayerControlled` Pawn)
    (bind _output_get (set `self.LastSeenActor` Pawn))
    (bind _asaicontroller_bp_hunter (cast `/Game/Blueprints/AI/AIController_BP_Hunter` (`self.GetController`)))
    (bind _returnvalue (`AIBlueprintHelperLibrary.GetBlackboard` _asaicontroller_bp_hunter))
    (`BlackboardComponent.SetValueAsObject` _returnvalue (`self.EnemyActor`) _output_get)
    (`BlackboardComponent.SetValueAsBool` _returnvalue (`self.HasLOS`) true)
    (`KismetSystemLibrary.K2_ClearAndInvalidateTimerHandle` (`self.VisionTimerHandle`))
    (`KismetSystemLibrary.K2_SetTimer` null "OnVisionMemoryExpired" (`self.VisionMemorySeconds`))))

(fn `ClearHeard`
  (cast `/Game/Blueprints/AI/AIController_BP_Hunter` (`self.GetController`))
  (`BlackboardComponent.ClearValue` (`AIBlueprintHelperLibrary.GetBlackboard` null) (`self.LastHeardLocation`)))

(fn `OnVisionMemoryExpired`
  (bind _asaicontroller_bp_hunter (cast `/Game/Blueprints/AI/AIController_BP_Hunter` (`self.GetController`)))
  (bind _returnvalue (`AIBlueprintHelperLibrary.GetBlackboard` _asaicontroller_bp_hunter))
  (`BlackboardComponent.ClearValue` _returnvalue (`self.EnemyActor`))
  (`BlackboardComponent.SetValueAsBool` _returnvalue (`self.HasLOS`) false)
  (set `self.LastSeenActor` null))

(fn `UserConstructionScript`)