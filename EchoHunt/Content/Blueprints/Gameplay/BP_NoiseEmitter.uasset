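; BP_NoiseEmitter is an interactable noise source that alerts enemy AI to its location.
; A character overlapping Box_Interact enables input on the actor, letting the E key trigger EmitNoise.
; EmitNoise writes the actor's location to the blackboard of each BP_Enemy controlled by AIController_BP_Hunter, using the NoiseVarName key.
; Each successful write also prints a debug message and draws a temporary debug sphere.
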(event `self.Box_Interact.OnComponentBeginOverlap`
  (params (OverlappedComponent :type "PrimitiveComponent Object Reference") (OtherActor :type "Actor Object Reference") (OtherComp :type "PrimitiveComponent Object Reference") (OtherBodyIndex :type Integer) (bFromSweep :type Boolean) (SweepResult :type "HitResult Structure (by ref)"))
  (if (`GameplayStatics.ObjectIsA` OtherActor "/Script/Engine.Character")
    (set `self.bPlayerInside` true)
    (`self.EnableInput` (`GameplayStatics.GetPlayerController` 0))))

(event `self.Box_Interact.OnComponentEndOverlap`
  (params (OverlappedComponent :type "PrimitiveComponent Object Reference") (OtherActor :type "Actor Object Reference") (OtherComp :type "PrimitiveComponent Object Reference") (OtherBodyIndex :type Integer))
  (if (`GameplayStatics.ObjectIsA` OtherActor "/Script/Engine.Character")
    (set `self.bPlayerInside` false)
    (`self.DisableInput` (`GameplayStatics.GetPlayerController` 0))))

(event `Key|E`
  (params (Key :type "Key Structure"))
  (:`Pressed`
    (if (`self.bPlayerInside`)
      (`self.EmitNoise`))))

(event `EmitNoise`
  (bind _output_get (set `self.NoiseLocation` (`self.K2_GetActorLocation`)))
  (bind _outactors (`GameplayStatics.GetAllActorsOfClass` "/Game/Blueprints/AI/BP_Enemy.BP_Enemy_C"))
  (for _array_element _outactors
    (bind _returnvalue (`AIBlueprintHelperLibrary.GetAIController` _array_element))
    (cast `/Game/Blueprints/AI/AIController_BP_Hunter` _returnvalue)
    (`BlackboardComponent.SetValueAsVector` (`AIBlueprintHelperLibrary.GetBlackboard` _returnvalue) (`self.NoiseVarName`) _output_get)
    (`KismetSystemLibrary.PrintString` "Noise Emitted")
    (`KismetSystemLibrary.DrawDebugSphere` (`self.NoiseLocation`) 50.0 12 (struct :`R` 1.0 :`B` 0.846547 :`A` 1.0) 2.0)))

(fn `UserConstructionScript`)